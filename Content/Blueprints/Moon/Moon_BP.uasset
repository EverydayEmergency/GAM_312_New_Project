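; Moon actor that fades the moon and its glow between day and night.
; NightTransition plays the DayToNight timeline to drive the Moon material's Opacity and the Glow's Density, and DayTransition reverses it.
; The construction script turns the actor to face an Origin point and applies a uniform Scale.
; A RotateAroundOrigin helper returns a point at a given rotation and distance from a center.
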(event `NightTransition`
  (bind (_direction _moon _glow) (`Timeline|DayToNight` :!label _label)
    (:`Update`
      (`MeshComponent.SetScalarParameterValueOnMaterials` (`self.Moon`) "Opacity" _moon)
      (`MeshComponent.SetScalarParameterValueOnMaterials` (`self.Glow`) "Density" _glow))))

(event `DayTransition`
  (goto _label :!via `Reverse`))

(fn `RotateAroundOrigin`
  (params (Center :type "Vector Structure") (Rotation :type "Rotator Structure") (Distance :type "Float (double-precision)"))
  (returns (ReturnValue :type "Vector Structure"))
  (return (+ Center (* (`KismetMathLibrary.GetForwardVector` Rotation) Distance))))

(fn `UserConstructionScript`
  (bind _scale (`self.Scale`))
  (`self.K2_SetActorRotation` (`KismetMathLibrary.Conv_VectorToRotator` (`KismetMathLibrary.Normal` (- (`self.Origin`) (`self.K2_GetActorLocation`)))))
  (`self.SetActorScale3D` (`KismetMathLibrary.MakeVector` _scale _scale _scale)))