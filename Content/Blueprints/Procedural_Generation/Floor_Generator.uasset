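; Procedural map generator that, on BeginPlay, builds and centers a grid of GrassFloor tiles, then populates it with objects and AI.
; Tiles chain along each row via their RightArrow, with barriers on outer edges made collidable and visibility-toggled.
; Each tile's SpawnFolder children form a shared pool, randomly consumed to place GatheringTypes, then raised AISpawned actors, by configured counts.
; AlterNavMesh scales the nav bounds to the grid but is never called here.
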(event `self.ReceiveBeginPlay`
  (bind _gatheringtypes (`self.GatheringTypes`))
  (bind _aispawned (`self.AISpawned`))
  ;[1 1 1 1 30] Event Beginplay
  (`self.Spawnmap`)
  (`self.Center Floors`)
  (bind _keys (`BlueprintMapLibrary.Map_Keys` _gatheringtypes))
  (for _array_element _keys
    (`self.Spawn Objects` (`BlueprintMapLibrary.Map_Find` _gatheringtypes _array_element) _array_element))
  (bind _keys_2 (`BlueprintMapLibrary.Map_Keys` _aispawned))
  (for _array_element_2 _keys_2
    (`self.SpawnAI` (`BlueprintMapLibrary.Map_Find` _aispawned _array_element_2) _array_element_2)))

(event `SetSpawnTransform`
  (bind _rowfloortile (`self.RowFloorTile`))
  (bind (_returnvalue_x _returnvalue_y) (`KismetMathLibrary.BreakVector` (`self.K2_GetActorLocation` _rowfloortile)))
  (bind (_returnvalue_x_2 _returnvalue_y_2) (`KismetMathLibrary.BreakVector` (`SceneComponent.K2_GetComponentScale` (`/Game/Blueprints/Procedural_Generation/MasterFloor_BP.Floor` _rowfloortile))))
  ;[0 1 0 1 30] Set Spawn Transform
  (set `self.Spawn Transform` (`KismetMathLibrary.MakeTransform` (`KismetMathLibrary.MakeVector` 0.0 (+ _returnvalue_y (* _returnvalue_y_2 100.0))))))

(event `CheckForBarrier`
  (params (FloorObj :type "/Game/Blueprints/Procedural_Generation/GrassFloor Object Reference") (IndexColumn :type Integer) (IndexRow :type Integer))
  (bind _indexcolumn (`self.IndexColumn`))
  (bind _floorobj (`self.FloorObj`))
  (bind _floorobj_2 (`self.FloorObj`))
  (bind _floorobj_3 (`self.FloorObj`))
  (bind _floorobj_4 (`self.FloorObj`))
  ;[0 1 0 1 30] Check for Barriers
  (set `self.FloorObj` FloorObj)
  (set `self.IndexColumn` IndexColumn)
  (set `self.IndexRow` IndexRow)
  (if (== _indexcolumn 0)
    (if (== (`self.IndexRow`) 0)
      (`self.MakeBarriers` (`/Game/Blueprints/Procedural_Generation/GrassFloor.LeftBarrier` _floorobj)) ; Create a barrier to the left
      (`self.MakeBarriers` (`/Game/Blueprints/Procedural_Generation/GrassFloor.UpBarrier` _floorobj)) ; Create an up barrier
      (elif (== (`self.IndexRow`) (- (`self.Floor Rows`) 1))
        (`self.MakeBarriers` (`/Game/Blueprints/Procedural_Generation/GrassFloor.RightBarrier` _floorobj_2)) ; Create a barrier to the right
        (`self.MakeBarriers` (`/Game/Blueprints/Procedural_Generation/GrassFloor.UpBarrier` _floorobj_2)) ; Create an up barrier
        (else
          (`self.MakeBarriers` (`/Game/Blueprints/Procedural_Generation/GrassFloor.UpBarrier` (`self.FloorObj`))) ; Create an up barrier
        )))
    (elif (== _indexcolumn (- (`self.Floor Columns`) 1))
      (if (== (`self.IndexRow`) (- (`self.Floor Rows`) 1))
        (`self.MakeBarriers` (`/Game/Blueprints/Procedural_Generation/GrassFloor.RightBarrier` _floorobj_4)) ; Create a barrier to the right
        (`self.MakeBarriers` (`/Game/Blueprints/Procedural_Generation/GrassFloor.DownBarrier` _floorobj_4)) ; Create a down barrier
        (elif (== (`self.IndexRow`) 0)
          (`self.MakeBarriers` (`/Game/Blueprints/Procedural_Generation/GrassFloor.LeftBarrier` _floorobj_3)) ; Create a barrier to the left
          (`self.MakeBarriers` (`/Game/Blueprints/Procedural_Generation/GrassFloor.DownBarrier` _floorobj_3)) ; Create a down barrier
          (else
            (`self.MakeBarriers` (`/Game/Blueprints/Procedural_Generation/GrassFloor.DownBarrier` (`self.FloorObj`))) ; Create a down barrier
          )))
      (elif (== (`self.IndexRow`) 0)
        (`self.MakeBarriers` (`/Game/Blueprints/Procedural_Generation/GrassFloor.LeftBarrier` (`self.FloorObj`))) ; Create a barrier to the left
        (elif (== (`self.IndexRow`) (- (`self.Floor Rows`) 1))
          (`self.MakeBarriers` (`/Game/Blueprints/Procedural_Generation/GrassFloor.RightBarrier` (`self.FloorObj`))) ; Create a barrier to the right
        )))))

(event `Add Floor Spawn Points`
  ;[0 1 0 1 30] Adds Spawn Points to List
  (`KismetArrayLibrary.Array_Append` (`self.FloorSpawnPoints`) (`SceneComponent.GetChildrenComponents` (`/Game/Blueprints/Procedural_Generation/MasterFloor_BP.Spawn Folder` (`self.CurrentFloor`)) false)))

(event `MakeBarriers`
  (params (Barrier :type "StaticMeshComponent Object Reference"))
  ;[0 1 0 1 30] Make Barriers
  (`SceneComponent.ToggleVisibility` Barrier false)
  (`PrimitiveComponent.SetCollisionEnabled` Barrier "QueryAndPhysics"))

(event `SpawnMap`
  ;[0 1 0 1 30] SpawnMap
  (for _index (range (`self.Floor Columns`))
    (for _index_2 (range (`self.Floor Rows`))
      (bind _returnvalue (`|SpawnActorFromClass` "/Game/Blueprints/Procedural_Generation/GrassFloor.GrassFloor_C" (`self.Spawn Transform`) "AlwaysSpawn" "OverrideRootScale" null null))
      (`self.CheckForBarrier` _returnvalue _index _index_2)
      (bind _output_get (set `self.CurrentFloor` _returnvalue))
      (`KismetArrayLibrary.Array_Add` (`self.FloorsList`) _output_get)
      (if (== _index_2 0)
        (set `self.RowFloorTile` _returnvalue))
      (set `self.Spawn Transform` (`SceneComponent.K2_GetComponentToWorld` (`/Game/Blueprints/Procedural_Generation/MasterFloor_BP.RightArrow` _returnvalue)))
      (`self.Add Floor Spawn Points`))
    (`self.SetSpawnTransform`)))

(event `Center Floors`
  (bind (_returnvalue_x _returnvalue_y) (`KismetMathLibrary.BreakVector` (`SceneComponent.K2_GetComponentScale` (`/Game/Blueprints/Procedural_Generation/MasterFloor_BP.Floor` (`self.RowFloorTile`)))))
  ;[0 1 0 1 30] Center Floors
  (set `self.FloorXSize` (* _returnvalue_x 100.0 (/ (`self.Floor Columns`) 2.0)))
  (set `self.FloorYSize` (* _returnvalue_y 100.0 (/ (`self.Floor Rows`) 2.0)))
  (for _array_element (`self.FloorsList`)
    (bind (_returnvalue_x_2 _returnvalue_y_2 _returnvalue_z) (`KismetMathLibrary.BreakVector` (`self.K2_GetActorLocation` _array_element)))
    (`self.K2_SetActorLocation` _array_element (`KismetMathLibrary.MakeVector` (- _returnvalue_x_2 (`self.FloorXSize`)) (- _returnvalue_y_2 (`self.FloorYSize`)) _returnvalue_z) false false)))

(event `AlterNavMesh`
  (bind (_relativescale3d_x _relativescale3d_y _relativescale3d_z) (`KismetMathLibrary.BreakVector` (`SceneComponent.RelativeScale3D` (`/Game/Blueprints/Procedural_Generation/MasterFloor_BP.Floor` (`self.RowFloorTile`)))))
  (bind _returnvalue (`GameplayStatics.GetActorOfClass` "/Script/NavigationSystem.NavMeshBoundsVolume"))
  (`self.SetActorScale3D` _returnvalue (`KismetMathLibrary.MakeVector` (* _relativescale3d_x (`self.Floor Columns`)) (* _relativescale3d_y (`self.Floor Rows`)) (+ _relativescale3d_z 2.0))))

(event `Spawn Objects`
  (params (`Spawn Amount` :type Integer) (SpawnedObjectType :type "Actor Class Reference"))
  ;[0 1 0 1 30] Spawn Objects
  (if (> `Spawn Amount` 0)
    (for _ (range 1 (+ `Spawn Amount` 1))
      (if (> (`KismetArrayLibrary.Array_Length` (`self.FloorSpawnPoints`)) 0)
        (bind _output_get (set `self.Selected Spawn Location` (`KismetArrayLibrary.Array_Random` (`self.FloorSpawnPoints`))))
        (`|SpawnActorFromClass` SpawnedObjectType (`KismetMathLibrary.MakeTransform` (`SceneComponent.K2_GetComponentLocation` _output_get)) "AlwaysSpawn" "OverrideRootScale" null null)
        (`KismetArrayLibrary.Array_RemoveItem` (`self.FloorSpawnPoints`) (`self.Selected Spawn Location`))))))

(event `SpawnAI`
  (params (`Spawn Amount` :type Integer) (SpawnedObjectType :type "Actor Class Reference"))
  ;[0 1 0 1 30] Spawn AI
  (if (> `Spawn Amount` 0)
    (for _ (range 1 (+ `Spawn Amount` 1))
      (if (> (`KismetArrayLibrary.Array_Length` (`self.FloorSpawnPoints`)) 0)
        (bind _output_get (set `self.Selected Spawn Location` (`KismetArrayLibrary.Array_Random` (`self.FloorSpawnPoints`))))
        (bind (_returnvalue_x _returnvalue_y _returnvalue_z) (`KismetMathLibrary.BreakVector` (`SceneComponent.K2_GetComponentLocation` _output_get)))
        (`|SpawnActorFromClass` SpawnedObjectType (`KismetMathLibrary.MakeTransform` (`KismetMathLibrary.MakeVector` _returnvalue_x _returnvalue_y (+ _returnvalue_z 150.0))) "AlwaysSpawn" "OverrideRootScale" null null)
        (`KismetArrayLibrary.Array_RemoveItem` (`self.FloorSpawnPoints`) (`self.Selected Spawn Location`))))))

(fn `UserConstructionScript`)